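; Player controller that turns input into camera look, movement and jumping for the controlled character.
; Forward movement follows a stored yaw-only rotation, updated toward control rotation through RInterpTo after each movement input.
; Strafe input blends that rotation's right vector with the pawn's facing and uses absolute axis magnitude, so sideways movement also carries forward.
; Two separate Turn axis events both add yaw input.
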(event `InputAction|Jump`
  (params (Key :type "Key Structure"))
  (:`Pressed`
    (bind _ascharacter (cast `Character` (`GameplayStatics.GetPlayerPawn` 0)))
    (`Character.Jump` _ascharacter)))

(event `InputAxis|LookUp`
  (params (AxisValue :type "Float (single-precision)"))
  (`self.AddPitchInput` AxisValue))

(event `InputAxis|Turn`
  (params (AxisValue :type "Float (single-precision)"))
  (`self.AddYawInput` AxisValue))

(event `InputAxis|MoveForward`
  (params (AxisValue :type "Float (single-precision)"))
  (bind (_returnvalue_roll _returnvalue_pitch _returnvalue_yaw) (`KismetMathLibrary.BreakRotator` (`KismetMathLibrary.RInterpTo` (`self.MovementRotationTarget`) (`self.GetControlRotation` (`GameplayStatics.GetPlayerController` 0)) (`GameplayStatics.GetWorldDeltaSeconds`))))
  (`Pawn.AddMovementInput` (`GameplayStatics.GetPlayerPawn` 0) (`KismetMathLibrary.GetForwardVector` (`self.MovementRotationTarget`)) AxisValue false)
  (set `self.MovementRotationTarget` (`KismetMathLibrary.MakeRotator` 0.0 0.0 _returnvalue_yaw)))

(event `InputAxis|MoveRight`
  (params (AxisValue :type "Float (single-precision)"))
  (bind (_returnvalue_roll _returnvalue_pitch _returnvalue_yaw) (`KismetMathLibrary.BreakRotator` (`self.K2_GetActorRotation` (`GameplayStatics.GetPlayerPawn` 0))))
  (`Pawn.AddMovementInput` (`GameplayStatics.GetPlayerPawn` 0) (`KismetMathLibrary.Normal` (+ (* AxisValue (`KismetMathLibrary.GetRightVector` (`self.MovementRotationTarget`))) (`KismetMathLibrary.GetForwardVector` (`KismetMathLibrary.MakeRotator` 0.0 0.0 _returnvalue_yaw)))) (`KismetMathLibrary.Abs` AxisValue) false))

(event `InputAxis|Turn`
  (params (AxisValue :type "Float (single-precision)"))
  (`self.AddYawInput` (`GameplayStatics.GetPlayerController` 0) AxisValue))

(fn `UserConstructionScript`)